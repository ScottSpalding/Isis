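; BP_GA_Tile_Square is a square tile Blueprint in the Advanced Turn Based Tile Toolkit that can switch between an opaque and a transparent look.
; MakeTransparent hides StaticMesh1 and shows TranslucentMesh, and Makeopaque reverses this.
; The switch toggles visibility on the two mesh components without propagating to children, so no material changes at runtime.
; The construction script only calls the parent's.
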(event `Make Transparent`
  (`SceneComponent.SetVisibility` (`self.StaticMesh1`) false false)
  (`SceneComponent.SetVisibility` (`self.TranslucentMesh`) true false))

(event `Make opaque`
  (`SceneComponent.SetVisibility` (`self.StaticMesh1`) true false)
  (`SceneComponent.SetVisibility` (`self.TranslucentMesh`) false false))

(fn `UserConstructionScript`
  (locals (`Opacity Material` :type "Array of MaterialInstanceDynamic Object Reference"))
  (`parent.UserConstructionScript`))