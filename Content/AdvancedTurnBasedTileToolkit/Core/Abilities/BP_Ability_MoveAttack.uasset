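; Turn-based unit ability that lets a unit move within range or make a ranged attack on a valid target.
; Remaining AP decides whether pathfinding shows move tiles, only attacks remain or the turn ends; hover previews paths and clicks execute.
; AI favors low-health targets, otherwise moving toward the closest relevant unit.
; Damage applies immediately while queued actions animate it later; BeginPlay also creates instanced cover meshes if a cover system exists.
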(event `Multicast_AssignCoverMesh`
  (bind _returnvalue (`self.GetComponentByClass` (`self.GridManagerRef`) "/Game/AdvancedTurnBasedTileToolkit/Core/Grid/BP_CoverSystem.BP_CoverSystem_C"))
  ;[1 1 1] Begin Play
  (bind _returnvalue_2 (`AddComponent|NODE_AddHierarchicalInstancedStaticMeshComponent-1`))
  (bind _output_get (set `/Game/AdvancedTurnBasedTileToolkit/Core/Grid/BP_CoverSystem.CoverHISM` _returnvalue_2 _returnvalue))
  (`StaticMeshComponent.SetStaticMesh` _output_get (`/Game/AdvancedTurnBasedTileToolkit/Core/Grid/BP_CoverSystem.CoverMesh` _returnvalue))
  (bind _returnvalue_3 (`AddComponent|NODE_AddHierarchicalInstancedStaticMeshComponent-2`))
  (bind _output_get_2 (set `/Game/AdvancedTurnBasedTileToolkit/Core/Grid/BP_CoverSystem.CoverHalfHISM` _returnvalue_3 _returnvalue))
  (`StaticMeshComponent.SetStaticMesh` _output_get_2 (`/Game/AdvancedTurnBasedTileToolkit/Core/Grid/BP_CoverSystem.CoverHalfMesh` _returnvalue)))

(event `self.ReceiveBeginPlay`
  (bind _gridmanagerref (`self.GridManagerRef`))
  ;[1 1 1] Begin Play
  (`parent.ReceiveBeginPlay`)
  (`/Game/AdvancedTurnBasedTileToolkit/Core/BPML_ATBTT.DelayWhile` (not (`KismetSystemLibrary.IsValid` _gridmanagerref))
    (:`Continue`
      (if (`KismetSystemLibrary.IsValid` (`self.GetComponentByClass` _gridmanagerref "/Game/AdvancedTurnBasedTileToolkit/Core/Grid/BP_CoverSystem.BP_CoverSystem_C"))
        (`self.Multicast_AssignCoverMesh`)))))

(event `self.FoundNoValidTarget`
  (bind _owningunit (`self.OwningUnit`))
  ;[0 0 0] AI
  (if (> (`/Game/AdvancedTurnBasedTileToolkit/Core/Units/BP_Unit.CurrentAP` (`self.OwningUnit`)) 1)
    (bind (_btargetfound _closestunitindex _btargetbehindfriendlyunit _distancetoclosesttarget _pathsmap) (`/Game/AdvancedTurnBasedTileToolkit/Core/Grid/BP_GridManager.FindClosestUnitInMoveRange` (`self.GridManagerRef`) (`/Game/AdvancedTurnBasedTileToolkit/Core/Units/BP_Unit.GridIndex` _owningunit) (`/Game/AdvancedTurnBasedTileToolkit/Core/Units/BP_Unit.MaxSearchRange` _owningunit) (`/Game/AdvancedTurnBasedTileToolkit/Core/Units/BP_Unit.PathfindingType` _owningunit) (`/Game/AdvancedTurnBasedTileToolkit/Core/Units/BP_Unit.AlliedFactions` _owningunit) true true))
    (if _btargetfound
      (bind _pathindexes (`/Game/AdvancedTurnBasedTileToolkit/Core/Grid/BP_GridManager.FindPathToIndex` (`self.GridManagerRef`) _pathsmap _closestunitindex))
      (bind (_bpathfound _closestindex) (`/Game/AdvancedTurnBasedTileToolkit/Core/Grid/BP_GridManager.FindReachableIndexClosestToTarget` (`self.GridManagerRef`) _pathindexes (`/Game/AdvancedTurnBasedTileToolkit/Core/Units/BP_Unit.PathfindingType` (`self.OwningUnit`)) (`self.PossibleMove`) _distancetoclosesttarget _pathsmap))
      (if _bpathfound
        (set `self.StoredPathsMap` _pathsmap)
        (set `self.MoveTargetIndex` _closestindex)
        (set `self.TargetIndex` -1)
        (`self.OnAbilityAssesmentDone` 0.001)
        (else
          (`self.OnAbilityAssesmentDone` 0.0)))
      (else
        (`self.OnAbilityAssesmentDone` 0.0)))
    (else
      (`self.OnAbilityAssesmentDone` 0.0))))

(event `self.Player_Activate`
  (params (Unit :type "/Game/AdvancedTurnBasedTileToolkit/Core/Units/BP_Unit Object Reference"))
  (bind _gridmanagerref (`self.GridManagerRef`))
  (bind _owningunit (`self.OwningUnit`))
  ;[0 0 0] Player Activate
  (switch `int` (`/Game/AdvancedTurnBasedTileToolkit/Core/Units/BP_Unit.CurrentAP` Unit)
    (:`Default`
      (set `self.bDisplayInvalidTiles` false)
      (`parent.Player_Activate` (`self.OwningUnit`))
      (bind _pathsmap (`/Game/AdvancedTurnBasedTileToolkit/Core/Grid/BP_GridManager.RunPathfinding` (`self.GridManagerRef`) (`/Game/AdvancedTurnBasedTileToolkit/Core/Units/BP_Unit.GridIndex` _owningunit) (`self.PossibleMove`) (`/Game/AdvancedTurnBasedTileToolkit/Core/Units/BP_Unit.PathfindingType` _owningunit)))
      (set `self.StoredPathsMap` _pathsmap)
      (`KismetArrayLibrary.Array_Clear` (`self.StoredLocations`))
      (bind _keys (`BlueprintMapLibrary.Map_Keys` (`self.StoredPathsMap`)))
      (if (> (`/Game/AdvancedTurnBasedTileToolkit/Core/Units/BP_Unit.Size` (`self.OwningUnit`)) 1)
        (bind _biggridindexes (`/Game/AdvancedTurnBasedTileToolkit/Core/Grid/BP_GridManager.FindBigIndexesFromIndexes` (`self.GridManagerRef`) _keys (`/Game/AdvancedTurnBasedTileToolkit/Core/Units/BP_Unit.Size` (`self.OwningUnit`))))
        (set `self.MoveDisplayIndexes` _biggridindexes)
        (else
          (set `self.MoveDisplayIndexes` _keys)))
      (for _array_element (`self.MoveDisplayIndexes`)
        (if (not (`BlueprintMapLibrary.Map_Contains` (`/Game/AdvancedTurnBasedTileToolkit/Core/Grid/BP_GridManager.GridUnits` (`self.GridManagerRef`)) _array_element))
          (bind _value (`BlueprintMapLibrary.Map_Find` (`/Game/AdvancedTurnBasedTileToolkit/Core/Grid/BP_GridManager.GridLocations` _gridmanagerref) _array_element))
          (`KismetArrayLibrary.Array_Add` (`self.StoredLocations`) (`KismetMathLibrary.MakeVector` (.x _value) (.y _value) (+ (.z _value) (`/Game/AdvancedTurnBasedTileToolkit/Core/Grid/BP_GridManager.TileInRangeZOffset` _gridmanagerref))))))
      (`/Game/AdvancedTurnBasedTileToolkit/Core/BPML_ATBTT.QueueAction` :`Executing Object` self :`Action Name` "DisplayMoveTiles" :`Instant Deactivate` true :`Vectors` (`self.StoredLocations`) :`Units` (`|MakeArray` (`self.OwningUnit`))))
    (:`0`
      (`/Game/AdvancedTurnBasedTileToolkit/Core/BP_TurnManager.EndTurn` (`/Game/AdvancedTurnBasedTileToolkit/Core/BP_ATBTT_State.TurnManager` (`self.GameStateRef`)) true true "NewEnumerator0" true true))
    (:`1`
      (set `self.bDisplayInvalidTiles` true)
      (`BlueprintMapLibrary.Map_Clear` (`self.StoredPathsMap`))
      (`parent.Player_Activate` (`self.OwningUnit`))
      (message `/Game/AdvancedTurnBasedTileToolkit/Core/BPI_Big.ToggleOffset` (`GameplayStatics.GetPlayerController` 0) false))))

(event `self.Click`
  (params (Index :type Integer) (Location :type "Vector Structure") (Key :type "Key Structure") (bReleased :type Boolean) (ClickType :type "/Game/AdvancedTurnBasedTileToolkit/Core/Grid/EClickType Enum" :default "NewEnumerator0"))
  (bind _owningunit (`self.OwningUnit`))
  (bind _owningunit_2 (`self.OwningUnit`))
  (bind _value (`BlueprintMapLibrary.Map_Find` (`self.StoredPathsMap`) (`self.TargetIndex`)))
  (bind (_value_2 _returnvalue) (`BlueprintMapLibrary.Map_Find` (`/Game/AdvancedTurnBasedTileToolkit/Core/Grid/BP_GridManager.GridUnits` (`self.GridManagerRef`)) (`self.TargetIndex`)))
  ;[0 0 0] Click
  (if (not bReleased)
    (switch `/Game/AdvancedTurnBasedTileToolkit/Core/Grid/EClickType` ClickType
      (:`NewEnumerator0`
        (set `self.TargetIndex` Index)
        (if (`BlueprintSetLibrary.Set_Contains` (`self.PossibleTargets`) (`self.TargetIndex`))
          (`self.PayAPCost` false)
          (`self.ExecuteAbility` (`self.TargetIndex`))
          (elif (and (>= (`self.PossibleMove`) (break `/Game/AdvancedTurnBasedTileToolkit/Core/Grid/FPathfindingNew` _value)) (> (break `/Game/AdvancedTurnBasedTileToolkit/Core/Grid/FPathfindingNew` _value) 0) (or (not _returnvalue) (and _returnvalue (== _value_2 _owningunit_2) (!= (`/Game/AdvancedTurnBasedTileToolkit/Core/Units/BP_Unit.GridIndex` _owningunit_2) (`self.TargetIndex`)))))
            (set `self.MoveTargetIndex` (`self.TargetIndex`))
            (`self.PayMoveAPCost`)
            (`self.ClickEmptyTile`)
            (elif _returnvalue
              (if (== (`BlueprintMapLibrary.Map_Find` (`/Game/AdvancedTurnBasedTileToolkit/Core/Grid/BP_GridManager.GridUnits` (`self.GridManagerRef`)) (`self.TargetIndex`)) (`self.OwningUnit`))
                (set `/Game/AdvancedTurnBasedTileToolkit/Core/Units/BP_Unit.CurrentAP` (`KismetMathLibrary.Max` (- (`/Game/AdvancedTurnBasedTileToolkit/Core/Units/BP_Unit.CurrentAP` _owningunit) 1)) _owningunit)
                (`/Game/AdvancedTurnBasedTileToolkit/Core/BP_TurnManager.ReactivateActiveUnit` (`/Game/AdvancedTurnBasedTileToolkit/Core/BP_ATBTT_State.TurnManager` (`self.GameStateRef`)))
                (else
                  (`self.DefaultClick` (`self.TargetIndex`) Location)))
              (elif (< (`/Game/AdvancedTurnBasedTileToolkit/Core/Units/BP_Unit.CurrentAP` (`self.OwningUnit`)) 2)
                (`self.DeactivateAbility`)
                (`/Game/AdvancedTurnBasedTileToolkit/Core/BP_TurnManager.EndTurn` (`/Game/AdvancedTurnBasedTileToolkit/Core/BP_ATBTT_State.TurnManager` (`self.GameStateRef`)) true true "NewEnumerator0" true true)))))))))

(event `self.ExecuteAbility`
  (params (TargetIndex :type Integer))
  ;[0 0 0] Click
  (`parent.ExecuteAbility` TargetIndex)
  (`/Game/AdvancedTurnBasedTileToolkit/Core/BPML_ATBTT.QueueAction` :`Executing Object` self :`Action Name` "Attack" :`Floats` (`|MakeArray` (`self.Damage`)) :`Units` (`|MakeArray` (`self.OwningUnit`) (`BlueprintMapLibrary.Map_Find` (`/Game/AdvancedTurnBasedTileToolkit/Core/Grid/BP_GridManager.GridUnits` (`self.GridManagerRef`)) (`self.TargetIndex`))))
  (`/Game/AdvancedTurnBasedTileToolkit/Core/Units/BP_Unit.TakeDamage` (`BlueprintMapLibrary.Map_Find` (`/Game/AdvancedTurnBasedTileToolkit/Core/Grid/BP_GridManager.GridUnits` (`self.GridManagerRef`)) (`self.TargetIndex`)) (`/Game/AdvancedTurnBasedTileToolkit/Core/Units/BP_Unit.Damage` (`self.OwningUnit`)) false)
  (`/Game/AdvancedTurnBasedTileToolkit/Core/BP_TurnManager.ReactivateActiveUnit` (`/Game/AdvancedTurnBasedTileToolkit/Core/BP_ATBTT_State.TurnManager` (`self.GameStateRef`))))

(event `ClickEmptyTile`
  (bind _value (`BlueprintMapLibrary.Map_Find` (`self.StoredPathsMap`) (`self.TargetIndex`)))
  ;[0 0 0] Click
  ;;[0 0.04285 0.515] Click Empty Tile
  ;;;[0 0 0] Prepare and Initialize Movement
  (if (and (>= (`self.PossibleMove`) (break `/Game/AdvancedTurnBasedTileToolkit/Core/Grid/FPathfindingNew` _value)) (> (break `/Game/AdvancedTurnBasedTileToolkit/Core/Grid/FPathfindingNew` _value) 0))
    (`self.ClearActivationMarkers`)
    (`/Game/AdvancedTurnBasedTileToolkit/Core/BPML_ATBTT.QueueAction` :`Executing Object` (`/Game/AdvancedTurnBasedTileToolkit/Core/BP_ATBTT_State.TurnManager` (`self.GameStateRef`)) :`Action Name` "SelectUnit" :`Instant Deactivate` true :`Units` (`|MakeArray` (`self.OwningUnit`)))
    (`/Game/AdvancedTurnBasedTileToolkit/Core/Units/BP_Unit.MoveToIndex` (`self.OwningUnit`) (`self.TargetIndex`) (`self.StoredPathsMap`))
    (if (`KismetSystemLibrary.IsValid` (`self.OwningUnit`))
      (`/Game/AdvancedTurnBasedTileToolkit/Core/BP_TurnManager.ReactivateActiveUnit` (`/Game/AdvancedTurnBasedTileToolkit/Core/BP_ATBTT_State.TurnManager` (`self.GameStateRef`))))))

(event `self.Hover`
  (params (Index :type Integer) (Location :type "Vector Structure"))
  (bind (_value _returnvalue) (`BlueprintMapLibrary.Map_Find` (`/Game/AdvancedTurnBasedTileToolkit/Core/Grid/BP_GridManager.GridUnits` (`self.GridManagerRef`)) (`self.HoveredTile`)))
  ;[0 0 0] Hover
  (`parent.Hover` Index Location)
  (`self.Client_ClearPath`)
  (if (>= Index 0)
    (if (`/Game/AdvancedTurnBasedTileToolkit/Core/Grid/BP_GridManager.IsTileImpassable` (`self.GridManagerRef`) (`self.HoveredTile`))
      _
      (elif _returnvalue
        (if (and (== (`self.OwningUnit`) _value) (!= (`/Game/AdvancedTurnBasedTileToolkit/Core/Units/BP_Unit.GridIndex` (`self.OwningUnit`)) (`self.HoveredTile`)))
          (if (`BlueprintMapLibrary.Map_Contains` (`self.StoredPathsMap`) (`self.HoveredTile`)) :!label _label
            (bind (_pathindexes _pathlocations) (`/Game/AdvancedTurnBasedTileToolkit/Core/Grid/BP_GridManager.FindAndDisplayPath` (`self.GridManagerRef`) (`self.StoredPathsMap`) (`self.HoveredTile`) false (`/Game/AdvancedTurnBasedTileToolkit/Core/Grid/BP_GridManager.bDisplayPathAsSpline` (`self.GridManagerRef`)) (`/Game/AdvancedTurnBasedTileToolkit/Core/Units/BP_Unit.BigUnitOffset` (`self.OwningUnit`)))) ; Find and show a path from the path hovered to the tile the pathfinding array was generated from (generally the current pawn)
            (`self.Client_DisplayPath` _pathlocations)))
        (else
          (goto _label))))))

(event `Client_DisplayPath`
  (params (PathLocations :type "Array of Vector Structure"))
  (bind _gridmanagerref (`self.GridManagerRef`))
  (bind _pathspline (`/Game/AdvancedTurnBasedTileToolkit/Core/Grid/BP_GridManager.PathSpline` (`self.GridManagerRef`)))
  ;[0 0 0] Hover
  (`SplineComponent.SetSplinePoints` _pathspline PathLocations "World" true)
  (if (`/Game/AdvancedTurnBasedTileToolkit/Core/Grid/BP_GridManager.bDisplayPathAsSpline` (`self.GridManagerRef`))
    (`/Game/AdvancedTurnBasedTileToolkit/Core/Grid/BP_GridManager.DisplayPathAsSpline` _gridmanagerref _pathspline PathLocations)
    (else
      (`/Game/AdvancedTurnBasedTileToolkit/Core/Grid/BP_GridManager.DisplayPathAsInstancedMeshes` _gridmanagerref PathLocations))))

(event `/Game/AdvancedTurnBasedTileToolkit/Core/BPI_Action.AnimateAction`
  (params (Action :type "/Game/AdvancedTurnBasedTileToolkit/Core/FAction Structure"))
  (bind (_executingobject _actionname _binstantdeactivate _atcustomindex _bwithprevious _activationdelay _booleans _integers _floats _strings _vectors _transforms _actors _units) (break `/Game/AdvancedTurnBasedTileToolkit/Core/FAction` Action))
  (bind _output (`|GetArrayItem` _units))
  ;[0 0 0] Animate Actions
  (switch `name` _actionname
    (:`Default`
      (`parent.AnimateAction` Action))
    (:`DisplayMoveTiles`
      (`self.SpawnTileMarkers` _output _vectors))
    (:`Attack`
      (`self.Attack` _output (`|GetArrayItem` _units 1) (`|GetArrayItem` _floats)))))

(event `SpawnTileMarkers`
  (params (OwningUnit :type "/Game/AdvancedTurnBasedTileToolkit/Core/Units/BP_Unit Object Reference") (Locations :type "Array of Vector Structure"))
  (bind _gridmanagerref (`self.GridManagerRef`))
  ;[0 0 0] Animate Actions
  ;;[0 0.2764 1] Spawn Tile Markers
  (`/Game/AdvancedTurnBasedTileToolkit/Core/BPML_ATBTT.OwnsUnit` OwningUnit
    (:`true`
      (`/Game/AdvancedTurnBasedTileToolkit/Core/Grid/BP_GridManager.SpawnTileMarkersAtLocations` (`self.GridManagerRef`) Locations (`/Game/AdvancedTurnBasedTileToolkit/Core/Grid/BP_GridManager.bUseDecals` _gridmanagerref) (`/Game/AdvancedTurnBasedTileToolkit/Core/Grid/BP_GridManager.TileInMoveRangeDecalT` _gridmanagerref) (`/Game/AdvancedTurnBasedTileToolkit/Core/Grid/BP_GridManager.TileInMoveRangeMC` _gridmanagerref)))))

(event `Client_SpawnCoverMeshes`
  (params (Array :type "Array of Transform Structure"))
  (bind _coverhism (`/Game/AdvancedTurnBasedTileToolkit/Core/Grid/BP_CoverSystem.CoverHISM` (`self.GetComponentByClass` (`self.GridManagerRef`) "/Game/AdvancedTurnBasedTileToolkit/Core/Grid/BP_CoverSystem.BP_CoverSystem_C")))
  ;[0 0 0] Hover
  (`InstancedStaticMeshComponent.ClearInstances` _coverhism)
  (for _array_element Array
    (`InstancedStaticMeshComponent.AddInstanceWorldSpace` _coverhism _array_element)))

(event `Client_HideTargetMarker`
  (bind _gridmanagerref (`self.GridManagerRef`))
  ;[0 0 0] Hover
  (`/Game/AdvancedTurnBasedTileToolkit/Core/Grid/BP_GridManager.SetMarkerVisibility` _gridmanagerref false (`/Game/AdvancedTurnBasedTileToolkit/Core/Grid/BP_GridManager.TargetMarkerDecal` _gridmanagerref) (`/Game/AdvancedTurnBasedTileToolkit/Core/Grid/BP_GridManager.TargetMarker` _gridmanagerref)))

(event `Attack`
  (params (Attacker :type "/Game/AdvancedTurnBasedTileToolkit/Core/Units/BP_Unit Object Reference") (TargetUnit :type "/Game/AdvancedTurnBasedTileToolkit/Core/Units/BP_Unit Object Reference") (Damage :type "Float (double-precision)"))
  ;[0 0 0] Animate Actions
  (add `/Game/AdvancedTurnBasedTileToolkit/Core/Units/BP_Unit.OnActionHit` Attacker (delegate `AttackHit`))
  (`/Game/AdvancedTurnBasedTileToolkit/Core/BPML_ATBTT.QueueAction` :`bImmediate` true :`Executing Object` Attacker :`Action Name` "ranged" :`Vectors` (`|MakeArray` (`self.K2_GetActorLocation` TargetUnit))))

(event `AttackHit`
  ;[0 0 0] Animate Actions
  (remove `/Game/AdvancedTurnBasedTileToolkit/Core/Units/BP_Unit.OnActionHit` (stale `Attack` Attacker) (delegate `AttackHit`))
  (`/Game/AdvancedTurnBasedTileToolkit/Core/Units/BP_Unit.AnimateTakeDamage` (stale `Attack` TargetUnit) (stale `Attack` Damage))
  (message `/Game/AdvancedTurnBasedTileToolkit/Core/BPI_Action.EndAction` (`GameplayStatics.GetGameState`)))

(event `self.DeactivateAbility`
  ;[0 0 0] Deactivate
  (`parent.DeactivateAbility`)
  (message `/Game/AdvancedTurnBasedTileToolkit/Core/BPI_Big.ToggleOffset` (`GameplayStatics.GetPlayerController` 0) false))

(fn `FindTargetValue`
  (params (TargetIndex :type Integer))
  (returns (Value :type "Float (double-precision)"))
  (return (/ 1.0 (`/Game/AdvancedTurnBasedTileToolkit/Core/Units/BP_Unit.CurrentHealth` (`BlueprintMapLibrary.Map_Find` (`/Game/AdvancedTurnBasedTileToolkit/Core/Grid/BP_GridManager.GridUnits` (`self.GridManagerRef`)) TargetIndex)))))

(fn `GetDescription`
  (returns (Description :type Text))
  (return "Move: \nMove to a tile within range."))

(fn `UserConstructionScript`
  (`parent.UserConstructionScript`))