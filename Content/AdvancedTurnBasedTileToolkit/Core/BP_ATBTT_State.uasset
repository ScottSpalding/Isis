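; Central state Blueprint for the Advanced Turn Based Tile Toolkit that creates and exposes the grid, turn and action managers.
; SetupCoreBlueprints finds the placed grid manager, spawns and initializes the turn manager, then spawns the action manager.
; It activates the grid manager last because grid setup needs the initiative order.
; It also forwards EndAction to the action manager and counts distinct unit owners in the initiative order.
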(event `/Game/AdvancedTurnBasedTileToolkit/Core/BPI_Action.EndAction`
  (`/Game/AdvancedTurnBasedTileToolkit/Core/BPI_Action.EndAction` (`self.ActionManager`)))

(fn `FindNumberOfUnitOwners`
  (returns (OwnerCount :type Integer))
  (locals (LocalOwningPlayers :type "Set of Integer"))
  (for _array_element (`/Game/AdvancedTurnBasedTileToolkit/Core/BP_TurnManager.InitiativeOrderUnits` (`self.TurnManager`))
    (bind _defaultowningplayer (`/Game/AdvancedTurnBasedTileToolkit/Core/Units/BP_Unit.DefaultOwningPlayer` _array_element))
    (if (not (`BlueprintSetLibrary.Set_Contains` (`local.LocalOwningPlayers`) _defaultowningplayer))
      (`BlueprintSetLibrary.Set_Add` (`local.LocalOwningPlayers`) _defaultowningplayer)))
  (return (`BlueprintSetLibrary.Set_Length` (`local.LocalOwningPlayers`))))

(fn `GetActionManager`
  (returns (ActionManader :type "/Game/AdvancedTurnBasedTileToolkit/Core/BP_ActionManager Object Reference"))
  (return (`self.ActionManager`)))

(fn `GetGridManager`
  (returns (GridManager :type "/Game/AdvancedTurnBasedTileToolkit/Core/Grid/BP_GridManager Object Reference"))
  (return (`self.GridManager`)))

(fn `GetTurnManager`
  (returns (TurnManager :type "/Game/AdvancedTurnBasedTileToolkit/Core/BP_TurnManager Object Reference"))
  (return (`self.TurnManager`)))

(fn `SetupCoreBlueprints`
  (bind _outactors (`GameplayStatics.GetAllActorsOfClass` "/Game/AdvancedTurnBasedTileToolkit/Core/Grid/BP_GridManager.BP_GridManager_C"))
  (set `self.GridManager` (`|GetArrayItem` _outactors))
  (bind _returnvalue (`|SpawnActorFromClass` "/Game/AdvancedTurnBasedTileToolkit/Core/BP_TurnManager.BP_TurnManager_C" (`KismetMathLibrary.MakeTransform` (0.0 0.0 0.0)) "AlwaysSpawn" "OverrideRootScale" null null))
  (bind _output_get (set `self.TurnManager` _returnvalue))
  (`/Game/AdvancedTurnBasedTileToolkit/Core/BP_TurnManager.Initialize` _output_get)
  (bind _returnvalue_2 (`|SpawnActorFromClass` "/Game/AdvancedTurnBasedTileToolkit/Core/BP_ActionManager.BP_ActionManager_C" (`KismetMathLibrary.MakeTransform` (0.0 0.0 0.0)) "AlwaysSpawn" "OverrideRootScale" null null))
  (set `self.ActionManager` _returnvalue_2)
  (`/Game/AdvancedTurnBasedTileToolkit/Core/Grid/BP_GridManager.ActivateGridManager` (`self.GridManager`)) ; Activate the grid manager after making the initiative order array, as this is used in the setup of BP_GridManager.
  (return))

(fn `UserConstructionScript`)