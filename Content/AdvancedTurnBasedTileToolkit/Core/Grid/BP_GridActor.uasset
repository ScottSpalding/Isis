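; BP_GridActor is an actor that registers its cell index on the tile grid and visually snaps to it at construction.
; The construction script finds BP_GridManager and converts the actor's location to GridIndex, using 3D or 2D conversion depending on the Heightmap setting.
; With grid snapping enabled and not ignored, it moves the mesh's GridAnchor to the cell location.
; PlaceActorAtAnchor acts as a one-shot toggle that moves the actor onto the anchor, then re-snaps.
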(fn `UserConstructionScript`
  (bind _outactors (`GameplayStatics.GetAllActorsOfClass` "/Game/AdvancedTurnBasedTileToolkit/Core/Grid/BP_GridManager.BP_GridManager_C")) ; Get a referance to the Grid Manager
  (set `self.GridManagerRef` (`|GetArrayItem` _outactors))
  (if (`|EnumEquality` (`/Game/AdvancedTurnBasedTileToolkit/Core/Grid/BP_GridManager.Heightmap` (`self.GridManagerRef`)) "NewEnumerator3")
    (bind (_bsuccess _index) (`/Game/AdvancedTurnBasedTileToolkit/Core/Grid/BP_GridManager.ConvertLocationToIndex3DNaive` (`self.GridManagerRef`) (`self.K2_GetActorLocation`)))
    (set `self.GridIndex` _index)
    (else
      (set `self.GridIndex` (`/Game/AdvancedTurnBasedTileToolkit/Core/Grid/BP_GridManager.ConvertLocationToIndex2D` (`self.GridManagerRef`) (`self.K2_GetActorLocation`)))))
  (if (`/Game/AdvancedTurnBasedTileToolkit/Core/Grid/BP_GridManager.bSnapToCustomGrid` (`self.GridManagerRef`))
    (if (not (`self.bIgnoreSnapToCustomGrid`))
      (bind (_bsuccess_2 _index_2 _location) (`/Game/AdvancedTurnBasedTileToolkit/Core/Grid/BP_GridManager.ConvertLocationToIndex3DNaive` (`self.GridManagerRef`) (`self.K2_GetActorLocation`) :!label _label))
      (`SceneComponent.K2_SetWorldLocation` (`self.GridAnchor`) _location false false) ; Set the location of the anchor which the mesh is tied to. Even though the actor is at the same position, the mesh will snap to the grid.
      (if (`self.bPlaceActorAtAnchor`)
        (`self.K2_SetActorLocation` (`SceneComponent.K2_GetComponentLocation` (`self.GridAnchor`)))
        (set `self.bPlaceActorAtAnchor` false)
        (goto _label)))))