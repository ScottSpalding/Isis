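; VR player class for the HTC Vive that lets the right motion controller act as the mouse in the turn-based tile game.
; On BeginPlay it sets floor tracking, waits for the turn manager, reports the player ready and starts a per-frame client loop.
; The loop traces from the right arrow, drawing a debug line, and sends hit locations to the player controller as hovers.
; Trigger press and release repeat the trace to send left-click messages.
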(event `ServerNotifyPlayerReady`
  (bind _turnmanager (message `/Game/AdvancedTurnBasedTileToolkit/Core/BPI_Singletons.GetTurnManager` (`GameplayStatics.GetGameState`)))
  (`/Game/AdvancedTurnBasedTileToolkit/Core/BPML_ATBTT.DelayWhile` (not (`KismetSystemLibrary.IsValid` _turnmanager))
    (:`Continue`
      (`/Game/AdvancedTurnBasedTileToolkit/Core/BP_TurnManager.NotifyPlayerReady` _turnmanager))))

(event `self.ReceiveBeginPlay`
  (`HeadMountedDisplayFunctionLibrary.SetTrackingOrigin` "Floor")
  (bind _turnmanager (message `/Game/AdvancedTurnBasedTileToolkit/Core/BPI_Singletons.GetTurnManager` (`GameplayStatics.GetGameState`)))
  (`/Game/AdvancedTurnBasedTileToolkit/Core/BPML_ATBTT.DelayWhile` (not (`KismetSystemLibrary.IsValid` _turnmanager))
    (:`Continue`
      (`self.ServerNotifyPlayerReady`)
      (`self.ClientBeginClientTick`))))

(event `ClientBeginClientTick`
  (bind _arrowright (`self.ArrowRight`))
  (bind _returnvalue (`SceneComponent.K2_GetComponentLocation` _arrowright))
  (`/Game/AdvancedTurnBasedTileToolkit/Core/BPML_ATBTT.WhileLoop_Delayed` (`self.bRunClientTick`)
    (:`Loop Body`
      (bind _outhit (`KismetSystemLibrary.LineTraceSingle` :`Start` _returnvalue :`End` (+ _returnvalue (* (`SceneComponent.GetForwardVector` _arrowright) 20000.0)) :`TraceChannel` "TraceTypeQuery3" :`DrawDebugType` "ForOneFrame"))
      (if (`GameplayStatics.BreakHitResult` _outhit)
        (message `/Game/AdvancedTurnBasedTileToolkit/Core/BPI_GridInteraction.Hover` (`GameplayStatics.GetPlayerController` 0) (`.Location` (`GameplayStatics.BreakHitResult` _outhit)))))))

(event `Key|MotionController_Right_Trigger`
  (params (Key :type "Key Structure"))
  (bind _arrowright (`self.ArrowRight`))
  (bind _returnvalue (`SceneComponent.K2_GetComponentLocation` _arrowright))
  (:`Pressed`
    (set `self.bReleased` false)
    (`GameplayStatics.PlaySound2D` "/Game/AdvancedTurnBasedTileToolkit/Core/Abilities/A_Discover.A_Discover")
    (bind (_outhit _returnvalue_2) (`KismetSystemLibrary.LineTraceSingle` _returnvalue (+ _returnvalue (* (`SceneComponent.GetForwardVector` _arrowright) 20000.0)) "TraceTypeQuery3" :!label _label))
    (if _returnvalue_2
      (message `/Game/AdvancedTurnBasedTileToolkit/Core/BPI_GridInteraction.Click` (`GameplayStatics.GetPlayerController` 0) (`.Location` (`GameplayStatics.BreakHitResult` _outhit)) "LeftMouseButton" (`self.bReleased`))))
  (:`Released`
    (set `self.bReleased` true)
    (goto _label)))

(fn `UserConstructionScript`)