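; Overwatch ability for the turn-based tile toolkit that readies a unit to fire at any enemy moving to a visible tile in range.
; Player activation pays the default AP cost and executes if the unit has AP left, otherwise it just reactivates the active unit.
; Execution applies BP_StatusEffect_Overwatch to the owning unit, then reactivates the active unit.
; The AssessAbilityValue event sets the default cooldown before calling its parent.
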(event `self.AssessAbilityValue`
  (params (Unit :type "/Game/AdvancedTurnBasedTileToolkit/Core/Units/BP_Unit Object Reference"))
  (set `self.DefaultCooldown` 2)
  (`parent.AssessAbilityValue` Unit))

(event `self.Player_Activate`
  (params (Unit :type "/Game/AdvancedTurnBasedTileToolkit/Core/Units/BP_Unit Object Reference"))
  ;[0.2284 1 0] Player Activate
  (if (> (`/Game/AdvancedTurnBasedTileToolkit/Core/Units/BP_Unit.CurrentAP` Unit) 0)
    (`self.PayAPCost` false)
    (`self.ExecuteAbility` (`self.TargetIndex`))
    (else
      (`/Game/AdvancedTurnBasedTileToolkit/Core/BP_TurnManager.ReactivateActiveUnit` (`/Game/AdvancedTurnBasedTileToolkit/Core/BP_ATBTT_State.TurnManager` (`self.GameStateRef`))))))

(event `self.ExecuteAbility`
  (params (TargetIndex :type Integer))
  ;[0 1 0.6707] Execute Ability
  (`parent.ExecuteAbility` TargetIndex)
  (`self.AddStatusEffect` "/Game/AdvancedTurnBasedTileToolkit/Maps/Advanced/Abilities/BP_StatusEffect_Overwatch.BP_StatusEffect_Overwatch_C" (`self.OwningUnit`))
  (`/Game/AdvancedTurnBasedTileToolkit/Core/BP_TurnManager.ReactivateActiveUnit` (`/Game/AdvancedTurnBasedTileToolkit/Core/BP_ATBTT_State.TurnManager` (`self.GameStateRef`))))

(fn `GetDescription`
  (returns (Description :type Text))
  (return (`KismetTextLibrary.Conv_StringToText` (`KismetStringLibrary.Concat_StrStr` (`KismetTextLibrary.Conv_TextToString` "Overwatch: \n") (`KismetTextLibrary.Conv_TextToString` "Fire at any anemy target that moves to a visible \ntile in range.")))))

(fn `UserConstructionScript`
  (`parent.UserConstructionScript`))