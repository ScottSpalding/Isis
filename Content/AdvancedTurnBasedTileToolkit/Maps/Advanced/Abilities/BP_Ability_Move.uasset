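; Move ability for the turn-based tile toolkit that moves a unit along the grid, spending AP per Move's worth of path cost.
; Player activation queues near/far range markers; hovering previews the path, nearby cover as HISM instances and crosshairs on potential targets visible from that tile.
; AI heads toward the closest relevant unit, then picks the reachable tile around that point with the lowest danger rating from BP_CoverSystem.
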(event `Multicast_AssignCoverMesh`
  (bind _returnvalue (`self.GetComponentByClass` (`self.GridManagerRef`) "/Game/AdvancedTurnBasedTileToolkit/Core/Grid/BP_CoverSystem.BP_CoverSystem_C"))
  ;[1 1 1] Begin Play
  (bind _returnvalue_2 (`AddComponent|NODE_AddHierarchicalInstancedStaticMeshComponent-1`))
  (bind _output_get (set `/Game/AdvancedTurnBasedTileToolkit/Core/Grid/BP_CoverSystem.CoverHISM` _returnvalue_2 _returnvalue))
  (`StaticMeshComponent.SetStaticMesh` _output_get (`/Game/AdvancedTurnBasedTileToolkit/Core/Grid/BP_CoverSystem.CoverMesh` _returnvalue))
  (bind _returnvalue_3 (`AddComponent|NODE_AddHierarchicalInstancedStaticMeshComponent-2`))
  (bind _output_get_2 (set `/Game/AdvancedTurnBasedTileToolkit/Core/Grid/BP_CoverSystem.CoverHalfHISM` _returnvalue_3 _returnvalue))
  (`StaticMeshComponent.SetStaticMesh` _output_get_2 (`/Game/AdvancedTurnBasedTileToolkit/Core/Grid/BP_CoverSystem.CoverHalfMesh` _returnvalue)))

(event `self.ReceiveBeginPlay`
  (bind _gridmanagerref (`self.GridManagerRef`))
  ;[1 1 1] Begin Play
  (`parent.ReceiveBeginPlay`)
  (`/Game/AdvancedTurnBasedTileToolkit/Core/BPML_ATBTT.DelayWhile` (not (`KismetSystemLibrary.IsValid` _gridmanagerref))
    (:`Continue`
      (if (`KismetSystemLibrary.IsValid` (`self.GetComponentByClass` _gridmanagerref "/Game/AdvancedTurnBasedTileToolkit/Core/Grid/BP_CoverSystem.BP_CoverSystem_C"))
        (`self.Multicast_AssignCoverMesh`)))))

(event `self.AssessAbilityValue`
  (params (Unit :type "/Game/AdvancedTurnBasedTileToolkit/Core/Units/BP_Unit Object Reference"))
  ;[0 0 0] AI
  (`self.OnAbilityAssesmentDone` 0.001))

(event `self.AI_Activate`
  (params (Unit :type "/Game/AdvancedTurnBasedTileToolkit/Core/Units/BP_Unit Object Reference"))
  (bind _owningunit (`self.OwningUnit`))
  (bind _owningunit_2 (`self.OwningUnit`))
  (bind _owningunit_3 (`self.OwningUnit`))
  (bind _owningunit_4 (`self.OwningUnit`))
  ;[0 0 0] AI
  (bind _bmeetsrequirements (`self.CheckRequirements`))
  (if _bmeetsrequirements
    (bind (_btargetfound _closestunitindex _btargetbehindfriendlyunit _distancetoclosesttarget _pathsmap) (`/Game/AdvancedTurnBasedTileToolkit/Core/Grid/BP_GridManager.FindClosestUnitInMoveRange` (`self.GridManagerRef`) (`/Game/AdvancedTurnBasedTileToolkit/Core/Units/BP_Unit.GridIndex` _owningunit_4) (`/Game/AdvancedTurnBasedTileToolkit/Core/Units/BP_Unit.MaxSearchRange` _owningunit_4) (`/Game/AdvancedTurnBasedTileToolkit/Core/Units/BP_Unit.PathfindingType` _owningunit_4) (`/Game/AdvancedTurnBasedTileToolkit/Core/Units/BP_Unit.AlliedFactions` _owningunit_4) true true))
    (if _btargetfound
      (bind _pathindexes (`/Game/AdvancedTurnBasedTileToolkit/Core/Grid/BP_GridManager.FindPathToIndex` (`self.GridManagerRef`) _pathsmap _closestunitindex))
      (bind (_bpathfound _closestindex) (`/Game/AdvancedTurnBasedTileToolkit/Core/Grid/BP_GridManager.FindReachableIndexClosestToTarget` (`self.GridManagerRef`) _pathindexes (`/Game/AdvancedTurnBasedTileToolkit/Core/Units/BP_Unit.PathfindingType` (`self.OwningUnit`)) (* (`/Game/AdvancedTurnBasedTileToolkit/Core/Units/BP_Unit.CurrentAP` _owningunit) (`/Game/AdvancedTurnBasedTileToolkit/Core/Units/BP_Unit.Move` _owningunit)) _distancetoclosesttarget _pathsmap))
      (if _bpathfound
        (set `self.StoredPathsMap` _pathsmap)
        (`KismetArrayLibrary.Array_Clear` (`self.AIMoveTargets`))
        (`KismetArrayLibrary.Array_Clear` (`self.AIMoveTargetValues`))
        (bind _pathsmap_2 (`/Game/AdvancedTurnBasedTileToolkit/Core/Grid/BP_GridManager.RunPathfinding` (`self.GridManagerRef`) _closestindex (`/Game/AdvancedTurnBasedTileToolkit/Core/Units/BP_Unit.Move` _owningunit_2) (`/Game/AdvancedTurnBasedTileToolkit/Core/Units/BP_Unit.PathfindingType` _owningunit_2)))
        (bind _keys (`BlueprintMapLibrary.Map_Keys` _pathsmap_2))
        (for _array_element _keys
          (bind _value (`BlueprintMapLibrary.Map_Find` (`self.StoredPathsMap`) _array_element))
          (if (or (and (> (break `/Game/AdvancedTurnBasedTileToolkit/Core/Grid/FPathfindingNew` _value) 0) (<= (break `/Game/AdvancedTurnBasedTileToolkit/Core/Grid/FPathfindingNew` _value) (* (`/Game/AdvancedTurnBasedTileToolkit/Core/Units/BP_Unit.CurrentAP` _owningunit_3) (`/Game/AdvancedTurnBasedTileToolkit/Core/Units/BP_Unit.Move` _owningunit_3))) (not (`BlueprintMapLibrary.Map_Contains` (`/Game/AdvancedTurnBasedTileToolkit/Core/Grid/BP_GridManager.GridUnits` (`self.GridManagerRef`)) _array_element))) (== _array_element (`/Game/AdvancedTurnBasedTileToolkit/Core/Units/BP_Unit.GridIndex` (`self.OwningUnit`))))
            (`KismetArrayLibrary.Array_Add` (`self.AIMoveTargets`) _array_element)
            (bind _value_2 (`/Game/AdvancedTurnBasedTileToolkit/Core/Grid/BP_CoverSystem.AssessTileDangerValue` (`self.GetComponentByClass` (`self.GridManagerRef`) "/Game/AdvancedTurnBasedTileToolkit/Core/Grid/BP_CoverSystem.BP_CoverSystem_C") _array_element (`/Game/AdvancedTurnBasedTileToolkit/Core/Units/BP_Unit.Faction` (`self.OwningUnit`))))
            (`KismetArrayLibrary.Array_Add` (`self.AIMoveTargetValues`) (- 1.0 _value_2))))
        (set `self.TargetIndex` (`|GetArrayItem` (`self.AIMoveTargets`) (`KismetMathLibrary.MaxOfFloatArray` (`self.AIMoveTargetValues`))))
        (if (!= (`/Game/AdvancedTurnBasedTileToolkit/Core/Units/BP_Unit.GridIndex` (`self.OwningUnit`)) (`self.TargetIndex`))
          (set `/Game/AdvancedTurnBasedTileToolkit/Core/Units/BP_Unit.CurrentAP` (`KismetMathLibrary.Max` (- (`/Game/AdvancedTurnBasedTileToolkit/Core/Units/BP_Unit.CurrentAP` (`self.OwningUnit`)) (+ (/ (- (break `/Game/AdvancedTurnBasedTileToolkit/Core/Grid/FPathfindingNew` (`BlueprintMapLibrary.Map_Find` (`self.StoredPathsMap`) (`self.TargetIndex`))) 1) (`/Game/AdvancedTurnBasedTileToolkit/Core/Units/BP_Unit.Move` (`self.OwningUnit`))) 1))) (`self.OwningUnit`))
          (`self.ExecuteAbility` (`self.TargetIndex`))
          (else
            (`self.FoundNoValidTarget`)))
        (else
          (`self.FoundNoValidTarget`)))
      (else
        (`self.FoundNoValidTarget`)))
    (else
      (`self.FoundNoValidTarget`))))

(event `self.FoundNoValidTarget`
  ;[0 0 0] AI
  (set `/Game/AdvancedTurnBasedTileToolkit/Core/Units/BP_Unit.CurrentAP` 0 (`self.OwningUnit`))
  (`/Game/AdvancedTurnBasedTileToolkit/Core/BP_TurnManager.ReactivateActiveUnit` (`/Game/AdvancedTurnBasedTileToolkit/Core/BP_ATBTT_State.TurnManager` (`self.GameStateRef`))))

(event `self.Player_Activate`
  (params (Unit :type "/Game/AdvancedTurnBasedTileToolkit/Core/Units/BP_Unit Object Reference"))
  (bind _nearlocations (`self.NearLocations`))
  (bind _gridmanagerref (`self.GridManagerRef`))
  (bind _owningunit (`self.OwningUnit`))
  ;[0 0 0] Player Activate
  (if (> (`/Game/AdvancedTurnBasedTileToolkit/Core/Units/BP_Unit.CurrentAP` Unit) 0)
    (bind _pathsmap (`/Game/AdvancedTurnBasedTileToolkit/Core/Grid/BP_GridManager.RunPathfinding` (`self.GridManagerRef`) (`/Game/AdvancedTurnBasedTileToolkit/Core/Units/BP_Unit.GridIndex` _owningunit) (* (`/Game/AdvancedTurnBasedTileToolkit/Core/Units/BP_Unit.CurrentAP` _owningunit) (`/Game/AdvancedTurnBasedTileToolkit/Core/Units/BP_Unit.Move` _owningunit)) (`/Game/AdvancedTurnBasedTileToolkit/Core/Units/BP_Unit.PathfindingType` _owningunit)))
    (set `self.StoredPathsMap` _pathsmap)
    (`KismetArrayLibrary.Array_Clear` (`self.NearLocations`))
    (`KismetArrayLibrary.Array_Clear` (`self.FarLocations`))
    (bind _keys (`BlueprintMapLibrary.Map_Keys` (`self.StoredPathsMap`)))
    (for _array_element _keys
      (if (`BlueprintMapLibrary.Map_Contains` (`/Game/AdvancedTurnBasedTileToolkit/Core/Grid/BP_GridManager.GridUnits` (`self.GridManagerRef`)) _array_element)
        _
        (elif (< (break `/Game/AdvancedTurnBasedTileToolkit/Core/Grid/FPathfindingNew` (`BlueprintMapLibrary.Map_Find` (`self.StoredPathsMap`) _array_element)) (+ (`/Game/AdvancedTurnBasedTileToolkit/Core/Units/BP_Unit.Move` (`self.OwningUnit`)) 1))
          (bind _value (`BlueprintMapLibrary.Map_Find` (`/Game/AdvancedTurnBasedTileToolkit/Core/Grid/BP_GridManager.GridLocations` _gridmanagerref) _array_element))
          (bind _returnvalue (`KismetMathLibrary.MakeVector` (.x _value) (.y _value) (+ (.z _value) (`/Game/AdvancedTurnBasedTileToolkit/Core/Grid/BP_GridManager.TileInRangeZOffset` _gridmanagerref))))
          (`KismetArrayLibrary.Array_Add` (`self.NearLocations`) _returnvalue)
          (else
            (`KismetArrayLibrary.Array_Add` (`self.FarLocations`) _returnvalue)))))
    (set `self.ArraySplitIndex` (`KismetArrayLibrary.Array_LastIndex` _nearlocations))
    (`KismetArrayLibrary.Array_Append` _nearlocations (`self.FarLocations`))
    (`/Game/AdvancedTurnBasedTileToolkit/Core/BPML_ATBTT.QueueAction` :`Executing Object` self :`Action Name` "DisplayMoveTiles" :`Instant Deactivate` true :`Integers` (`|MakeArray` (`self.ArraySplitIndex`)) :`Vectors` (`self.NearLocations`) :`Units` (`|MakeArray` (`self.OwningUnit`)))
    (else
      (`/Game/AdvancedTurnBasedTileToolkit/Core/BP_TurnManager.EndTurn` (`/Game/AdvancedTurnBasedTileToolkit/Core/BP_ATBTT_State.TurnManager` (`self.GameStateRef`)) true true "NewEnumerator0" true true))))

(event `self.Click`
  (params (Index :type Integer) (Location :type "Vector Structure") (Key :type "Key Structure") (bReleased :type Boolean) (ClickType :type "/Game/AdvancedTurnBasedTileToolkit/Core/Grid/EClickType Enum" :default "NewEnumerator0"))
  ;[0 0 0] Click
  (set `self.TargetIndex` Index)
  (if (`BlueprintMapLibrary.Map_Contains` (`/Game/AdvancedTurnBasedTileToolkit/Core/Grid/BP_GridManager.GridUnits` (`self.GridManagerRef`)) (`self.TargetIndex`))
    (`self.DefaultClick` (`self.TargetIndex`))
    (else
      (`self.ClickEmptyTile`))))

(event `ClickEmptyTile`
  (bind _owningunit (`self.OwningUnit`))
  (bind _value (`BlueprintMapLibrary.Map_Find` (`self.StoredPathsMap`) (`self.TargetIndex`)))
  ;[0 0 0] Click
  ;;[0 0.04285 0.515] Click Empty Tile
  ;;;[0 0 0] Prepare and Initialize Movement
  (if (and (>= (* (`/Game/AdvancedTurnBasedTileToolkit/Core/Units/BP_Unit.CurrentAP` _owningunit) (`/Game/AdvancedTurnBasedTileToolkit/Core/Units/BP_Unit.Move` _owningunit)) (break `/Game/AdvancedTurnBasedTileToolkit/Core/Grid/FPathfindingNew` _value)) (> (break `/Game/AdvancedTurnBasedTileToolkit/Core/Grid/FPathfindingNew` _value) 0))
    (set `/Game/AdvancedTurnBasedTileToolkit/Core/Units/BP_Unit.CurrentAP` (`KismetMathLibrary.Max` (- (`/Game/AdvancedTurnBasedTileToolkit/Core/Units/BP_Unit.CurrentAP` (`self.OwningUnit`)) (+ (/ (- (break `/Game/AdvancedTurnBasedTileToolkit/Core/Grid/FPathfindingNew` (`BlueprintMapLibrary.Map_Find` (`self.StoredPathsMap`) (`self.TargetIndex`))) 1) (`/Game/AdvancedTurnBasedTileToolkit/Core/Units/BP_Unit.Move` (`self.OwningUnit`))) 1))) (`self.OwningUnit`))
    (`self.ExecuteAbility` (`self.TargetIndex`))))

(event `self.ExecuteAbility`
  (params (TargetIndex :type Integer))
  ;[0 0 0] Click
  ;;[0 0.04285 0.515] Click Empty Tile
  (`parent.ExecuteAbility` TargetIndex)
  (`/Game/AdvancedTurnBasedTileToolkit/Core/BPML_ATBTT.QueueAction` :`Executing Object` (`/Game/AdvancedTurnBasedTileToolkit/Core/BP_ATBTT_State.TurnManager` (`self.GameStateRef`)) :`Action Name` "SelectUnit" :`Instant Deactivate` true :`Units` (`|MakeArray` (`self.OwningUnit`)))
  (`/Game/AdvancedTurnBasedTileToolkit/Core/Units/BP_Unit.MoveToIndex` (`self.OwningUnit`) (`self.TargetIndex`) (`self.StoredPathsMap`))
  (if (`KismetSystemLibrary.IsValid` (`self.OwningUnit`))
    (`/Game/AdvancedTurnBasedTileToolkit/Core/BP_TurnManager.ReactivateActiveUnit` (`/Game/AdvancedTurnBasedTileToolkit/Core/BP_ATBTT_State.TurnManager` (`self.GameStateRef`)))))

(event `self.Hover`
  (params (Index :type Integer) (Location :type "Vector Structure"))
  (bind _owningunit (`self.OwningUnit`))
  ;[0 0 0] Hover
  (`parent.Hover` Index Location)
  (`self.Client_ClearPath`)
  (`self.ClientClearCoverMeshes`)
  (if (>= Index 0)
    (bind _insightunits (`/Game/AdvancedTurnBasedTileToolkit/Core/Grid/BP_GridManager.FindVisibleUnitsInRange` (`self.GridManagerRef`) Index 20 false (* 20 (`/Game/AdvancedTurnBasedTileToolkit/Core/Grid/BP_GridManager.TileXSize` (`self.GridManagerRef`))) 0))
    (bind (_bfoundvalidtargets _outindexes) (`/Game/AdvancedTurnBasedTileToolkit/Core/Grid/BP_GridManager.KeepIndexesWithRelevantUnitsSet` (`self.GridManagerRef`) _insightunits (`/Game/AdvancedTurnBasedTileToolkit/Core/Units/BP_Unit.AlliedFactions` _owningunit) true true _owningunit))
    (if _bfoundvalidtargets
      (bind _units (`/Game/AdvancedTurnBasedTileToolkit/Core/Grid/BP_GridManager.GetUnitsFromGridIndexSet` (`self.GridManagerRef`) _outindexes))
      (bind _result (`BlueprintSetLibrary.Set_ToArray` _units))
      (`self.ClientShowCrosshairsOnPotentialUnits` _result)
      (else
        (`self.ClientClearCrosshairs`)))
    (bind (_fullcovertransforms _halfcovertransforms) (`/Game/AdvancedTurnBasedTileToolkit/Core/Grid/BP_CoverSystem.GetCoverMesheTransformsAroundIndex` (`self.GetComponentByClass` (`self.GridManagerRef`) "/Game/AdvancedTurnBasedTileToolkit/Core/Grid/BP_CoverSystem.BP_CoverSystem_C") (`self.HoveredTile`)))
    (`self.Client_SpawnCoverMeshes` _fullcovertransforms _halfcovertransforms)
    (if (`/Game/AdvancedTurnBasedTileToolkit/Core/Grid/BP_GridManager.IsTileImpassable` (`self.GridManagerRef`) (`self.HoveredTile`))
      _
      (elif (`BlueprintMapLibrary.Map_Contains` (`/Game/AdvancedTurnBasedTileToolkit/Core/Grid/BP_GridManager.GridUnits` (`self.GridManagerRef`)) (`self.HoveredTile`))
        _
        (elif (> (break `/Game/AdvancedTurnBasedTileToolkit/Core/Grid/FPathfindingNew` (`BlueprintMapLibrary.Map_Find` (`self.StoredPathsMap`) (`self.HoveredTile`))) 0)
          (bind (_pathindexes _pathlocations) (`/Game/AdvancedTurnBasedTileToolkit/Core/Grid/BP_GridManager.FindAndDisplayPath` (`self.GridManagerRef`) (`self.StoredPathsMap`) (`self.HoveredTile`) false (`/Game/AdvancedTurnBasedTileToolkit/Core/Grid/BP_GridManager.bDisplayPathAsSpline` (`self.GridManagerRef`)) (`/Game/AdvancedTurnBasedTileToolkit/Core/Units/BP_Unit.BigUnitOffset` (`self.OwningUnit`)))) ; Find and show a path from the path hovered to the tile the pathfinding array was generated from (generally the current pawn)
          (`self.Client_DisplayPath` _pathlocations))))
    (else
      (`self.ClientClearCrosshairs`))))

(event `Client_DisplayPath`
  (params (PathLocations :type "Array of Vector Structure"))
  (bind _pathspline (`/Game/AdvancedTurnBasedTileToolkit/Core/Grid/BP_GridManager.PathSpline` (`self.GridManagerRef`)))
  ;[0 0 0] Animate Actions
  (`SplineComponent.SetSplinePoints` _pathspline PathLocations "World" true)
  (`/Game/AdvancedTurnBasedTileToolkit/Core/Grid/BP_GridManager.DisplayPathAsSpline` (`self.GridManagerRef`) _pathspline PathLocations))

(event `/Game/AdvancedTurnBasedTileToolkit/Core/BPI_Action.AnimateAction`
  (params (Action :type "/Game/AdvancedTurnBasedTileToolkit/Core/FAction Structure"))
  (bind (_executingobject _actionname _binstantdeactivate _atcustomindex _bwithprevious _activationdelay _booleans _integers _floats _strings _vectors _transforms _actors _units) (break `/Game/AdvancedTurnBasedTileToolkit/Core/FAction` Action))
  ;[0 0 0] Animate Actions
  (switch `name` _actionname
    (:`Default`
      (`parent.AnimateAction` Action))
    (:`DisplayMoveTiles`
      (`self.SpawnTileMarkers` (`|GetArrayItem` _units) _vectors (`|GetArrayItem` _integers)))))

(event `SpawnTileMarkers`
  (params (OwningUnit :type "/Game/AdvancedTurnBasedTileToolkit/Core/Units/BP_Unit Object Reference") (Locations :type "Array of Vector Structure") (NearFarSplit :type Integer))
  (bind _gridmanagerref (`self.GridManagerRef`))
  (bind _gridmanagerref_2 (`self.GridManagerRef`))
  ;[0 0 0] Animate Actions
  ;;[0 0.2764 1] Spawn Tile Markers
  (`/Game/AdvancedTurnBasedTileToolkit/Core/BPML_ATBTT.OwnsUnit` OwningUnit
    (:`true`
      (bind (_zerotosplit _splittolast) (`/Game/AdvancedTurnBasedTileToolkit/Core/BPML_ATBTT.SplitArray` Locations NearFarSplit)
        (:` `
          (`/Game/AdvancedTurnBasedTileToolkit/Core/Grid/BP_GridManager.SpawnTileMarkersAtLocations` (`self.GridManagerRef`) _zerotosplit (`/Game/AdvancedTurnBasedTileToolkit/Core/Grid/BP_GridManager.bUseDecals` _gridmanagerref) (`/Game/AdvancedTurnBasedTileToolkit/Core/Grid/BP_GridManager.TileInMoveRangeDecalT` _gridmanagerref) (`/Game/AdvancedTurnBasedTileToolkit/Core/Grid/BP_GridManager.TileInMoveRangeMC` _gridmanagerref))
          (`/Game/AdvancedTurnBasedTileToolkit/Core/Grid/BP_GridManager.SpawnTileMarkersAtLocations` (`self.GridManagerRef`) _splittolast (`/Game/AdvancedTurnBasedTileToolkit/Core/Grid/BP_GridManager.bUseDecals` _gridmanagerref_2) (`/Game/AdvancedTurnBasedTileToolkit/Core/Grid/BP_GridManager.TileInLongMoveRangeDecalT` _gridmanagerref_2) (`/Game/AdvancedTurnBasedTileToolkit/Core/Grid/BP_GridManager.TileInLongMoveRangeMC` _gridmanagerref_2)))))))

(event `Client_SpawnCoverMeshes`
  (params (FullCoverTransforms :type "Array of Transform Structure") (HalfCoverTransforms :type "Array of Transform Structure"))
  (bind _returnvalue (`self.GetComponentByClass` (`self.GridManagerRef`) "/Game/AdvancedTurnBasedTileToolkit/Core/Grid/BP_CoverSystem.BP_CoverSystem_C"))
  (bind _coverhism (`/Game/AdvancedTurnBasedTileToolkit/Core/Grid/BP_CoverSystem.CoverHISM` _returnvalue))
  ;[0 0 0] Display Cover Meshes
  (`InstancedStaticMeshComponent.ClearInstances` _coverhism)
  (`InstancedStaticMeshComponent.ClearInstances` (`/Game/AdvancedTurnBasedTileToolkit/Core/Grid/BP_CoverSystem.CoverHalfHISM` _returnvalue))
  (for _array_element FullCoverTransforms
    (`InstancedStaticMeshComponent.AddInstanceWorldSpace` _coverhism _array_element))
  (for _array_element_2 HalfCoverTransforms
    (`InstancedStaticMeshComponent.AddInstanceWorldSpace` (`/Game/AdvancedTurnBasedTileToolkit/Core/Grid/BP_CoverSystem.CoverHalfHISM` _returnvalue) _array_element_2)))

(event `Client_HideTargetMarker`
  (bind _gridmanagerref (`self.GridManagerRef`))
  ;[0 0 0] Display Cover Meshes
  (`/Game/AdvancedTurnBasedTileToolkit/Core/Grid/BP_GridManager.SetMarkerVisibility` _gridmanagerref false (`/Game/AdvancedTurnBasedTileToolkit/Core/Grid/BP_GridManager.TargetMarkerDecal` _gridmanagerref) (`/Game/AdvancedTurnBasedTileToolkit/Core/Grid/BP_GridManager.TargetMarker` _gridmanagerref)))

(event `ClientShowCrosshairsOnPotentialUnits`
  (params (Units :type "Array of /Game/AdvancedTurnBasedTileToolkit/Core/Units/BP_Unit Object Reference (by ref)"))
  ;[0 0 0] Display Cover Meshes
  (`/Game/AdvancedTurnBasedTileToolkit/Core/Grid/BP_GridManager.ShowCrosshairsOnUnits` (`self.GridManagerRef`) Units))

(event `ClientClearCoverMeshes`
  ;[0 0 0] Display Cover Meshes
  (`InstancedStaticMeshComponent.ClearInstances` (`/Game/AdvancedTurnBasedTileToolkit/Core/Grid/BP_CoverSystem.CoverHISM` (`self.GetComponentByClass` (`self.GridManagerRef`) "/Game/AdvancedTurnBasedTileToolkit/Core/Grid/BP_CoverSystem.BP_CoverSystem_C")))
  (`InstancedStaticMeshComponent.ClearInstances` (`/Game/AdvancedTurnBasedTileToolkit/Core/Grid/BP_CoverSystem.CoverHalfHISM` (`self.GetComponentByClass` (`self.GridManagerRef`) "/Game/AdvancedTurnBasedTileToolkit/Core/Grid/BP_CoverSystem.BP_CoverSystem_C"))))

(event `self.ClearMeshes`
  ;[0 0 0] Display Cover Meshes
  (`parent.ClearMeshes`)
  (`self.ClientClearCoverMeshes`)
  (`self.ClientClearCrosshairs`))

(event `ClientClearCrosshairs`
  ;[0 0 0] Display Cover Meshes
  (`/Game/AdvancedTurnBasedTileToolkit/Core/Grid/BP_GridManager.RemoveCrosshairs` (`self.GridManagerRef`)))

(event `self.DeactivateAbility`
  ;[0 0 0] Deactivate
  (`parent.DeactivateAbility`)
  (if (!= (`self.BigUnitOffset`) (0.0 0.0 0.0))
    (set `self.BigUnitOffset` (0.0 0.0 0.0))
    (bind _asbp_player_controller_atbtt (cast `/Game/AdvancedTurnBasedTileToolkit/Core/BP_PlayerController_ATBTT` (`GameplayStatics.GetPlayerController` 0)))
    (set `/Game/AdvancedTurnBasedTileToolkit/Core/BP_PlayerController_ATBTT.BigUnitOffset` (0.0 0.0 0.0) _asbp_player_controller_atbtt)))

(fn `FindTargetValue`
  (params (TargetIndex :type Integer))
  (returns (Value :type "Float (double-precision)"))
  (return (/ 1.0 (`/Game/AdvancedTurnBasedTileToolkit/Core/Units/BP_Unit.CurrentHealth` (`BlueprintMapLibrary.Map_Find` (`/Game/AdvancedTurnBasedTileToolkit/Core/Grid/BP_GridManager.GridUnits` (`self.GridManagerRef`)) TargetIndex)))))

(fn `GetDescription`
  (returns (Description :type Text))
  (return "Move: \nMove to a tile within range."))

(fn `GetHoverText`
  (returns (HoverText :type Text))
  (bind _value (`BlueprintMapLibrary.Map_Find` (`self.StoredPathsMap`) (`self.HoveredTile`)))
  (if (`BlueprintMapLibrary.Map_Contains` (`/Game/AdvancedTurnBasedTileToolkit/Core/Grid/BP_GridManager.GridUnits` (`self.GridManagerRef`)) (`self.HoveredTile`))
    (return "Move: \nAP Cost: -")
    (else
      (return (`KismetTextLibrary.Conv_StringToText` (`KismetStringLibrary.Concat_StrStr` "Move: \nAP Cost: " (`KismetMathLibrary.SelectString` (`KismetStringLibrary.Conv_IntToString` (+ (/ (break `/Game/AdvancedTurnBasedTileToolkit/Core/Grid/FPathfindingNew` _value) (+ (`/Game/AdvancedTurnBasedTileToolkit/Core/Units/BP_Unit.Move` (`self.OwningUnit`)) 1)) 1)) "-" (> (break `/Game/AdvancedTurnBasedTileToolkit/Core/Grid/FPathfindingNew` _value) 0))))))))

(fn `UserConstructionScript`
  (`parent.UserConstructionScript`))