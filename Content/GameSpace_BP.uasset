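; GameSpace_BP is a game space square actor that highlights when the cursor hovers over it.
; BeginPlay enables input and mouse-over events, hides the cursor and creates a dynamic material instance on GameSpaceSquare.
; Cursor-over events switch that material's Color parameter between yellow and grey, while the click handler is empty.
; PointArrowAtLocation spawns a Pointer actor at a given transform, and an unconnected check would hide the square when pawns are present.
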(event `self.ReceiveBeginPlay`
  (bind _returnvalue (`GameplayStatics.GetPlayerController` 0))
  (`self.EnableInput` _returnvalue)
  (set `PlayerController.bEnableMouseOverEvents` true _returnvalue)
  (set `PlayerController.bShowMouseCursor` false _returnvalue)
  (bind _returnvalue_2 (`PrimitiveComponent.CreateDynamicMaterialInstance` (`self.GameSpaceSquare`) 0 "/Game/Assets/Materials/NewMaterial.NewMaterial")))

(event `self.GameSpaceSquare.OnBeginCursorOver`
  (params (TouchedComponent :type "PrimitiveComponent Object Reference"))
  (`MaterialInstanceDynamic.SetVectorParameterValue` (stale `self.ReceiveBeginPlay` _returnvalue_2) "Color" (struct :`R` 0.833333 :`G` 0.815881 :`B` 0.100867 :`A` 1.0)))

(event `self.GameSpaceSquare.OnEndCursorOver`
  (params (TouchedComponent :type "PrimitiveComponent Object Reference"))
  (`MaterialInstanceDynamic.SetVectorParameterValue` (stale `self.ReceiveBeginPlay` _returnvalue_2) "Color" (struct :`R` 0.453125 :`G` 0.453125 :`B` 0.453125 :`A` 1.0)))

(event `self.GameSpaceSquare.OnClicked`
  (params (TouchedComponent :type "PrimitiveComponent Object Reference") (ButtonPressed :type "Key Structure")))

(event `self.ReceiveTick`
  (params (DeltaSeconds :type "Float (single-precision)")))

(fn `Point Arrow At Location`
  (params (`Spawn Transform` :type "Transform Structure"))
  (`|SpawnActorFromClass` "/Game/Debug/Pointer.Pointer_C" `Spawn Transform` "Undefined" "OverrideRootScale" null null))

(fn `UserConstructionScript`)