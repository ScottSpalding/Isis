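; Game state Blueprint whose Initialize sets up the play grid and places a pawn on it.
; It spawns and activates a grid manager without diagonal movement, then spawns an IsisPawn and registers it on the grid.
; Registration and each location axis use separate random rolls over nine indices, so they can disagree.
; Disconnected nodes for spawning an enemy and seeding game spaces with random items never run.
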(fn `Initialize`
  (locals (NewLocalVar_0 :type "/Game/AdvancedTurnBasedTileToolkit/Core/Grid/BP_GridManager Object Reference") (NewLocalVar_1 :type "Vector Structure" :default (0.0 0.0 0.0)))
  (bind _returnvalue (`KismetMathLibrary.RandomInteger` 9))
  (bind _value (`BlueprintMapLibrary.Map_Find` (`/Game/AdvancedTurnBasedTileToolkit/Core/Grid/BP_GridManager.GridLocations` (`self.BP Grid Manager Ref`)) _returnvalue))
  (bind _returnvalue_2 (`|SpawnActorFromClass` "/Game/AdvancedTurnBasedTileToolkit/Core/Grid/BP_GridManager.BP_GridManager_C" (`KismetMathLibrary.Conv_VectorToTransform` (0.0 0.0 0.0)) "Undefined" "OverrideRootScale" null 3 3 false true true "NewEnumerator0" false 100.0 100.0 1000.0 0.0 false false 200.0 5 true null))
  (bind _output_get (set `self.BP Grid Manager Ref` _returnvalue_2))
  (`/Game/AdvancedTurnBasedTileToolkit/Core/Grid/BP_GridManager.ActivateGridManager` _output_get)
  (bind _returnvalue_3 (`|SpawnActorFromClass` "/Game/IsisPawn_BP.IsisPawn_BP_C" (`KismetMathLibrary.Conv_VectorToTransform` (500.0 500.0 500.0)) "Undefined" "OverrideRootScale" null 2 2 6 1 0 100.0 100.0 35.0 false "NewEnumerator0" true null))
  (bind _output_get_2 (set `/Game/AdvancedTurnBasedTileToolkit/Core/Units/BP_Unit.GridManagerRef` (`self.BP Grid Manager Ref`) _returnvalue_3))
  (`/Game/AdvancedTurnBasedTileToolkit/Core/Grid/BP_GridManager.AddUnitToGrid` _output_get_2 _returnvalue _returnvalue_3)
  (`self.K2_SetActorLocation` _returnvalue_3 (`KismetMathLibrary.MakeVector` (.x _value) (.y _value) (+ (.z _value) (`CapsuleComponent.GetScaledCapsuleHalfHeight` (`Character.CapsuleComponent` _returnvalue_3)))) false false))

(fn `UserConstructionScript`)