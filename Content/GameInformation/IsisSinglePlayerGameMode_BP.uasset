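; Single-player game mode that builds the 3x3 game board at BeginPlay and enables mouse click and hover events.
; It spawns nine game spaces in a grid, links orthogonal neighbours both ways with arrows pointing at each other, and makes the centre the board's core space.
; It then registers the board with IsisGameState_BP, spawns an enemy in a random location and adds three random items to every space.
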(event `self.ReceiveBeginPlay`
  (bind _returnvalue (`GameplayStatics.GetPlayerController` 0))
  (`parent.ReceiveBeginPlay`)
  (`self.EnableInput` _returnvalue)
  (set `PlayerController.bEnableClickEvents` true _returnvalue)
  (set `PlayerController.bEnableMouseOverEvents` true _returnvalue)
  (cast `/Game/GameInformation/IsisGameState_BP` (`GameplayStatics.GetGameState`))
  (bind _returnvalue_2 (`|SpawnActorFromClass` "/Game/Board/GameSpace_BP.GameSpace_BP_C" (`KismetMathLibrary.MakeTransform` (-525.0 525.0 0.0) (struct) (5.0 5.0 1.0)) "Undefined" "OverrideRootScale" null null))
  (bind _returnvalue_3 (`|SpawnActorFromClass` "/Game/Board/GameSpace_BP.GameSpace_BP_C" (`KismetMathLibrary.MakeTransform` (-525.0 0.0 0.0) (struct) (5.0 5.0 1.0)) "Undefined" "OverrideRootScale" null null))
  (`self.Add Adjacent Game Space Double-Linked` _returnvalue_2 _returnvalue_3)
  (bind _returnvalue_4 (`|SpawnActorFromClass` "/Game/Board/GameSpace_BP.GameSpace_BP_C" (`KismetMathLibrary.MakeTransform` (-525.0 -525.0 0.0) (struct) (5.0 5.0 1.0)) "Undefined" "OverrideRootScale" null null))
  (`self.Add Adjacent Game Space Double-Linked` _returnvalue_4 _returnvalue_3)
  (bind _returnvalue_5 (`|SpawnActorFromClass` "/Game/Board/GameSpace_BP.GameSpace_BP_C" (`KismetMathLibrary.MakeTransform` (0.0 525.0 0.0) (struct) (5.0 5.0 1.0)) "Undefined" "OverrideRootScale" null null))
  (`self.Add Adjacent Game Space Double-Linked` _returnvalue_2 _returnvalue_5)
  (bind _returnvalue_6 (`|SpawnActorFromClass` "/Game/Board/GameSpace_BP.GameSpace_BP_C" (`KismetMathLibrary.MakeTransform` (0.0 0.0 0.0) (struct) (5.0 5.0 1.0)) "Undefined" "OverrideRootScale" null null))
  (`self.Add Adjacent Game Space Double-Linked` _returnvalue_3 _returnvalue_6)
  (`self.Add Adjacent Game Space Double-Linked` _returnvalue_5 _returnvalue_6)
  (bind _returnvalue_7 (`|SpawnActorFromClass` "/Game/Board/GameSpace_BP.GameSpace_BP_C" (`KismetMathLibrary.MakeTransform` (0.0 -525.0 0.0) (struct) (5.0 5.0 1.0)) "Undefined" "OverrideRootScale" null null))
  (`self.Add Adjacent Game Space Double-Linked` _returnvalue_4 _returnvalue_7)
  (`self.Add Adjacent Game Space Double-Linked` _returnvalue_7 _returnvalue_6)
  (bind _returnvalue_8 (`|SpawnActorFromClass` "/Game/Board/GameSpace_BP.GameSpace_BP_C" (`KismetMathLibrary.MakeTransform` (525.0 525.0 0.0) (struct) (5.0 5.0 1.0)) "Undefined" "OverrideRootScale" null null))
  (`self.Add Adjacent Game Space Double-Linked` _returnvalue_8 _returnvalue_5)
  (bind _returnvalue_9 (`|SpawnActorFromClass` "/Game/Board/GameSpace_BP.GameSpace_BP_C" (`KismetMathLibrary.MakeTransform` (525.0 0.0 0.0) (struct) (5.0 5.0 1.0)) "Undefined" "OverrideRootScale" null null))
  (`self.Add Adjacent Game Space Double-Linked` _returnvalue_6 _returnvalue_9)
  (`self.Add Adjacent Game Space Double-Linked` _returnvalue_9 _returnvalue_8)
  (bind _returnvalue_10 (`|SpawnActorFromClass` "/Game/Board/GameSpace_BP.GameSpace_BP_C" (`KismetMathLibrary.MakeTransform` (525.0 -525.0 0.0) (struct) (5.0 5.0 1.0)) "Undefined" "OverrideRootScale" null null))
  (`self.Add Adjacent Game Space Double-Linked` _returnvalue_10 _returnvalue_7)
  (`self.Add Adjacent Game Space Double-Linked` _returnvalue_9 _returnvalue_10)
  (bind _returnvalue_11 (`|SpawnActorFromClass` "/Game/Board/GameBoardThreeByThree_BP.GameBoardThreeByThree_BP_C" (`KismetMathLibrary.Conv_VectorToTransform` (0.0 0.0 0.0)) "Undefined" "OverrideRootScale" null null))
  (`GameBoard.AddGameSpace` _returnvalue_11 _returnvalue_2)
  (`GameBoard.AddGameSpace` _returnvalue_11 _returnvalue_3)
  (`GameBoard.AddGameSpace` _returnvalue_11 _returnvalue_4)
  (`GameBoard.AddGameSpace` _returnvalue_11 _returnvalue_5)
  (`GameBoard.AddGameSpace` _returnvalue_11 _returnvalue_6)
  (`GameBoard.AddGameSpace` _returnvalue_11 _returnvalue_7)
  (`GameBoard.AddGameSpace` _returnvalue_11 _returnvalue_8)
  (`GameBoard.AddGameSpace` _returnvalue_11 _returnvalue_9)
  (`GameBoard.AddGameSpace` _returnvalue_11 _returnvalue_10)
  (`GameBoard.SetCoreGameSpace` _returnvalue_11 _returnvalue_6)
  (bind _asisis_game_state_bp (cast `/Game/GameInformation/IsisGameState_BP` (`GameplayStatics.GetGameState`)))
  (`IsisGameState.SetCurrentGameBoard` _asisis_game_state_bp _returnvalue_11)
  (`self.SpawnNewEnemyInRandomLocation`)
  (bind _result (`BlueprintSetLibrary.Set_ToArray` (`GameBoard.GetAllGameSpaces` _returnvalue_11)))
  (for _array_element _result
    (bind _returnvalue_12 (`self.GetRandomItemFromAllAvailable`))
    (`GameSpace.AddPresentItem` _array_element _returnvalue_12)
    (bind _returnvalue_13 (`self.GetRandomItemFromAllAvailable`))
    (`GameSpace.AddPresentItem` _array_element _returnvalue_13)
    (bind _returnvalue_14 (`self.GetRandomItemFromAllAvailable`))
    (`GameSpace.AddPresentItem` _array_element _returnvalue_14))
  (`KismetSystemLibrary.PrintString` "Finished!"))

(fn `Add Adjacent Game Space Double-Linked`
  (params (`First Space` :type "GameSpace Object Reference") (`Second Space` :type "GameSpace Object Reference"))
  (bind _returnvalue (`self.K2_GetActorLocation` `First Space`))
  (bind _returnvalue_2 (`self.K2_GetActorLocation` `Second Space`))
  (`GameSpace.AddAdjacentGameSpace` `First Space` `Second Space`)
  (`GameSpace.AddAdjacentGameSpace` `Second Space` `First Space`)
  (bind _asgame_space_bp (cast `/Game/Board/GameSpace_BP` `First Space`))
  (`/Game/Board/GameSpace_BP.Point Arrow At Location` _asgame_space_bp (`KismetMathLibrary.MakeTransform` _returnvalue (`KismetMathLibrary.FindLookAtRotation` _returnvalue _returnvalue_2)))
  (bind _asgame_space_bp_2 (cast `/Game/Board/GameSpace_BP` `Second Space`))
  (`/Game/Board/GameSpace_BP.Point Arrow At Location` _asgame_space_bp_2 (`KismetMathLibrary.MakeTransform` _returnvalue_2 (`KismetMathLibrary.FindLookAtRotation` _returnvalue_2 _returnvalue))))

(fn `UserConstructionScript`
  (`parent.UserConstructionScript`))