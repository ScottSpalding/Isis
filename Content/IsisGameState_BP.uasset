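; Game state Blueprint for a board game that supplies the squares where players may legally start.
; GetPlayerStartSquares takes every space on the current game board, casts each to GameSpace_BP and collects those flagged IsLegalPlayerStart into the returned list.
; The event graph and construction script hold no logic.
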(event `self.ReceiveBeginPlay`)

(fn `GetPlayerStartSquares`
  (returns (LegalPlayerStarts :type "Set of /Game/GameSpace_BP Object Reference"))
  (bind _returnvalue (`self.GetCurrentGameBoard`))
  (bind _result (`BlueprintSetLibrary.Set_ToArray` (`GameBoard.GetAllGameSpaces` _returnvalue)))
  (for _array_element _result
    (bind _asgame_space_bp (cast `/Game/GameSpace_BP` _array_element))
    (if (`/Game/GameSpace_BP.IsLegalPlayerStart` _asgame_space_bp)
      (`BlueprintSetLibrary.Set_Add` (`self.LegalGameSpace`) _asgame_space_bp)))
  (return (`self.LegalGameSpace`)))

(fn `UserConstructionScript`)